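; BP_TimeMaster is a game clock actor that drives a day/night cycle by rotating the level's directional light.
; Tick accumulates elapsed seconds from a start hour, scaled by an adjustable speed multiplier and halted while paused.
; A looping timer broadcasts hour, minute and day fraction, then sets sun pitch by linearly mapping elapsed time against sunrise and sunset.
; The RemapValueToRange helper is not called here; that mapping is computed inline.
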(event Custom|Notify
  (bind _sunriseseconds (Variables|Default|GetSunRiseSeconds))
  (Variables|Default|SetCurHour (Math|Integer|%(Integer) (Math|Float|Truncate (/ (Variables|Default|GetElapsedSeconds) 3.6e+03)) 24))
  (Variables|Default|SetCurMin (Math|Float|Truncate (/ (Math|Float|%(Float) (Variables|Default|GetElapsedSeconds) 3.6e+03) 6e+01)))
  (Default|CallNotifyTime (Variables|Default|GetCurHour) (Variables|Default|GetCurMin) (Math|Float|%(Float) (/ (Variables|Default|GetElapsedSeconds) 8.64e+04) 1.0))
  (bind _output_get (Variables|Default|SetsunRotation (Math|Float|%(Float) (+ 1.8e+02 (* (/ (- (Variables|Default|GetElapsedSeconds) _sunriseseconds) (- (Variables|Default|GetSunSetSeconds) _sunriseseconds)) (- 3.6e+02 1.8e+02))) 3.6e+02)))
  (Transformation|SetActorRotation (Variables|Default|GetDirLight) (Math|Rotator|MakeRotator 0.0 _output_get 0.0)))

(event Custom|UpdateTimeSpeed
  (params (GameSpeedMult :type Float%20%28double-precision%29))
  (Variables|Default|SetGameSpeedMult GameSpeedMult))

(event EventTick
  (params (DeltaSeconds :type Float%20%28single-precision%29))
  (if (not (Variables|Default|GetIsPaused))
    (Variables|Default|SetElapsedSeconds (Math|Float|Max(Float) (+ (* DeltaSeconds (Variables|Default|GetGameSpeedMult)) (Variables|Default|GetElapsedSeconds)) 0.0))))

(event EventBeginPlay
  (bind _returnvalue (Actor|GetActorOfClass "/Script/Engine.DirectionalLight"))
  (bind _output_get (Variables|Default|SetDirLight _returnvalue))
  (Transformation|SetActorRotation _output_get)
  (Variables|Default|SetElapsedSeconds (* (Variables|Default|GetStartAtHour) 3.6e+03))
  (bind _returnvalue_2 (Utilities|Time|SetTimerbyEvent (delegate Custom|Notify) (Variables|Default|GetInitialTimeUpdateRate) true))
  (Variables|Default|SetTimeUpdateTimer _returnvalue_2))

(fn ConstructionScript)

(fn RemapValuetoRange
  (params (input :type Float%20%28double-precision%29) (input%20low :type Float%20%28double-precision%29) (input%20high :type Float%20%28double-precision%29) (Target%20low :type Float%20%28double-precision%29) (target%20high :type Float%20%28double-precision%29))
  (bind _returnvalue (Math|Float|MakeLiteralFloat Target%20low))
  (bind _returnvalue_2 (Math|Float|MakeLiteralFloat input%20low))
  (return (+ (* (/ (- (Math|Float|MakeLiteralFloat input) _returnvalue_2) (- (Math|Float|MakeLiteralFloat input%20high) _returnvalue_2)) (- (Math|Float|MakeLiteralFloat target%20high) _returnvalue)) _returnvalue)))