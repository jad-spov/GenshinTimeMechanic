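; Analog clock actor that shows the current time from BP_TimeOfDay on rotating hour and minute hands.
; On BeginPlay it finds BP_TimeOfDay if unassigned, then polls it on a looping timer.
; The authority converts time to hand yaws, with an optional hard-ticking hour hand, and multicasts the rotation.
; The construction script tints each hand through a dynamic material instance.
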(event Custom|RotateClock
  (params (HoursYaw :type Float%20%28double-precision%29) (MinutesYaw :type Float%20%28double-precision%29))
  ;[0 1 0.1542 0.82] Rotate Clock (multicast)
  (Utilities|FlowControl|Sequence
    (:then_0
      (Transformation|SetRelativeRotation (Variables|Default|GetHours) (Math|Rotator|MakeRotator 0.0 0.0 HoursYaw) false false))
    (:then_1
      (Transformation|SetRelativeRotation (Variables|Default|GetMinutes) (Math|Rotator|MakeRotator 0.0 0.0 MinutesYaw) false false))))

(event Custom|ResetUpdate
  (bind _bp_timeofday (Variables|Default|GetBP_TimeOfDay))
  (bind (_hour _minute _second) (Default|GetTime _bp_timeofday))
  (bind _returnvalue (Math|Conversions|ToFloat(Integer) _minute))
  (bind _returnvalue_2 (Math|Conversions|ToFloat(Integer) _second))
  (bind _returnvalue_3 (/ _returnvalue_2 6e+01))
  (bind _returnvalue_4 (+ _returnvalue _returnvalue_3))
  (bind _returnvalue_5 (/ _returnvalue_4 6e+01))
  ;[0 0.3517 1 0.82] Initializer
  (Utilities|FlowControl|DoOnce false) ; enters at Reset
)

(event Custom|UpdateClock
  (bind _bp_timeofday (Variables|Default|GetBP_TimeOfDay))
  (bind (_hour _minute _second) (Default|GetTime _bp_timeofday))
  (bind _returnvalue (Math|Conversions|ToFloat(Integer) _minute))
  (bind _returnvalue_2 (Math|Conversions|ToFloat(Integer) _second))
  (bind _returnvalue_3 (/ _returnvalue_2 6e+01))
  (bind _returnvalue_4 (+ _returnvalue _returnvalue_3))
  (bind _returnvalue_5 (/ _returnvalue_4 6e+01))
  ;[0 0.3517 1 0.82] Initializer
  (Networking|SwitchHasAuthority
    (:Authority
      (Utilities|FlowControl|DoOnce false
        (:Completed
          (CallFunction|RotateClock (* (/ (+ (|ConvertTo12HourFormat _hour) (Math|Float|SelectFloat 0.0 _returnvalue_5 (Variables|Default|GetHardTickHourHand?))) 12.0) 3.6e+02) (* _returnvalue_5 3.6e+02))
          (CallFunction|ResetUpdate))))))

(event EventBeginPlay
  ;[0 0.3517 1 0.82] Initializer
  (|GetTimeofDayBP)
  ;;[0 0 0 0.82] You can also control the notification from this end instead of depending on the event notifier method.
  (Utilities|Time|SetTimerbyEvent (delegate Custom|UpdateClock) (Variables|Default|GetClockUpdateSpeed) true))

(fn ConstructionScript
  (Utilities|SetClockHandColor (Variables|Default|GetHoursHand) (Variables|Default|GetColorHourHand))
  (Utilities|SetClockHandColor (Variables|Default|GetMinutesHand) (Variables|Default|GetColorMinuteHand)))