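; BP_TimeOfDay_ClockDigital is a placeable digital clock that shows the BP_TimeOfDay time as colored, sized 3D text.
; On BeginPlay it uses the assigned BP_TimeOfDay or finds one, printing a warning if none exists, and binds to its time notifications.
; The authority picks a 24-hour or 12-hour timestamp, optionally with AM/PM, and multicasts it to the text.
; A DoOnce with a short delay throttles updates.
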(event Custom|TryUpdateClock
  (params (NotifyData :type ST%20Notify%20Data%20Structure))
  (bind _time (Utilities|Struct|BreakST_NotifyData NotifyData))
  (bind (_timestamp12_withampm _timestamp12_noampm _timestamp24) (Utilities|Struct|BreakST_NotifyData_Time _time))
  ;[0 0.3517 1 0.82] Initializer
  (Networking|SwitchHasAuthority
    (:Authority
      ;;[0 0 0 0.82] We can use Do Once and a delay to optimize the frequencey of requests if we have a high notify rate but don't really need it at this end.
      (Utilities|FlowControl|DoOnce false :!label _label
        (:Completed
          (CallFunction|UpdateClock (select (Variables|Default|Getis12HourClock?) (select (Variables|Default|GetshowAMPM?) _timestamp12_withampm _timestamp12_noampm) _timestamp24))
          (Utilities|FlowControl|Delay 0.5)
          (goto _label Reset))))))

(event Custom|UpdateClock
  (params (Timestamp :type Text))
  ;[0 1 0.1542 0.82] Update Clock Timestamp (multicast)
  (Rendering|Components|TextRender|SetText (Variables|Default|GetTimestamp) Timestamp))

(event EventBeginPlay
  ;[0 0.3517 1 0.82] Initializer
  (|GetTimeofDayBP)
  (EventDispatchers|BindEventtoNotifyTime (Variables|Default|GetBP_TimeOfDay) (delegate Custom|TryUpdateClock)))

(fn ConstructionScript
  (Rendering|Components|TextRender|SetTextRenderColor (Variables|Default|GetTimestamp) (Variables|Default|GetColor))
  (Rendering|Components|TextRender|SetWorldSize (Variables|Default|GetTimestamp) (Variables|Default|GetFontSize)))