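; Level actor that swaps its linked daytime and nighttime light sources on and off as BP_TimeOfDay crosses day and night start times.
; On BeginPlay it finds the time-of-day actor, warns on screen about missing setup, and binds to time notifications.
; The server evaluates each notification, using paired DoOnce nodes that reset each other so lights toggle once per transition.
; A multicast event applies visibility to each light component.
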(event Custom|TryLightSwitch
  (params (NotifyData :type ST%20Notify%20Data%20Structure))
  (bind _time (Utilities|Struct|BreakST_NotifyData NotifyData))
  (bind (_hour24 _minute _second) (Utilities|Struct|BreakST_NotifyData_Time _time))
  ;[0 0.3517 1 0.82] Initializer
  (Networking|SwitchHasAuthority
    (:Authority
      (if (.isDaytime (Default|IsTimeOfDay (Variables|TimeOfDay-LightSwitchConfiguration|GetTimeOfDayBP) _hour24 _minute _second (Variables|TimeOfDay-LightSwitchConfiguration|GetDaytimeStartsAt) (Variables|TimeOfDay-LightSwitchConfiguration|GetNighttimeStartsAt))) ; Is it daytime?
        (Utilities|FlowControl|DoOnce false :!label _label
          (:Completed
            (CallFunction|ToggleLights true (Variables|TimeOfDay-LightSwitchConfiguration|GetDaytimeLights))
            (CallFunction|ToggleLights false (Variables|TimeOfDay-LightSwitchConfiguration|GetNighttimeLights))
            (goto _label_2 Reset)))
        (else
          (Utilities|FlowControl|DoOnce false :!label _label_2
            (:Completed
              (CallFunction|ToggleLights true (Variables|TimeOfDay-LightSwitchConfiguration|GetNighttimeLights))
              (CallFunction|ToggleLights false (Variables|TimeOfDay-LightSwitchConfiguration|GetDaytimeLights))
              (goto _label Reset))))))))

(event Custom|ToggleLights
  (params (Turn%20on? :type Boolean) (Lights :type Array%20of%20Light%20Object%20References))
  ;[0 1 0.1542 0.82] Toggle Lights (multicast)
  (for _array_element Lights
    (Utilities|IsValid _array_element
      (:Is%20Valid
        (Rendering|SetVisibility (Variables|/Script/Engine.Light|GetLightComponent _array_element) Turn%20on? false)))))

(event EventBeginPlay
  (bind _timeofdaybp (Variables|TimeOfDay-LightSwitchConfiguration|GetTimeOfDayBP))
  ;[0 0.3517 1 0.82] Initializer
  (|CheckforTimeOfDayBP)
  (|CheckforLights)
  (EventDispatchers|BindEventtoNotifyTime _timeofdaybp (delegate Custom|TryLightSwitch))
  (if (.isDaytime (Default|IsTimeOfDay _timeofdaybp (.Hour24 (Utilities|Struct|BreakST_NotifyData_Time (Utilities|Struct|BreakST_NotifyData (stale Custom|TryLightSwitch NotifyData)))) (.Minute (Utilities|Struct|BreakST_NotifyData_Time (Utilities|Struct|BreakST_NotifyData (stale Custom|TryLightSwitch NotifyData)))) (.Second (Utilities|Struct|BreakST_NotifyData_Time (Utilities|Struct|BreakST_NotifyData (stale Custom|TryLightSwitch NotifyData)))) (Variables|TimeOfDay-LightSwitchConfiguration|GetDaytimeStartsAt) (Variables|TimeOfDay-LightSwitchConfiguration|GetNighttimeStartsAt))) ; Is it daytime?
    (Utilities|FlowControl|DoOnce false :!label _label
      (:Completed
        (CallFunction|ToggleLights true (Variables|TimeOfDay-LightSwitchConfiguration|GetDaytimeLights))
        (CallFunction|ToggleLights false (Variables|TimeOfDay-LightSwitchConfiguration|GetNighttimeLights))
        (goto _label_2 Reset)))
    (else
      (Utilities|FlowControl|DoOnce false :!label _label_2
        (:Completed
          (CallFunction|ToggleLights true (Variables|TimeOfDay-LightSwitchConfiguration|GetNighttimeLights))
          (CallFunction|ToggleLights false (Variables|TimeOfDay-LightSwitchConfiguration|GetDaytimeLights))
          (goto _label Reset))))))

(fn ConstructionScript)