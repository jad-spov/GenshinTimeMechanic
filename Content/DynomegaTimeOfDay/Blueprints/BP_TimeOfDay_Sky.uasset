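; BP_TimeOfDay_Sky is a sky rotator that turns sun and optional moon directional lights with the day cycle from BP_TimeOfDay.
; At BeginPlay it checks references, printing warnings if missing, optionally aligns both lights, and caches their starting rotations.
; On each time notification, the server adds day-progress degrees to each starting pitch, zeroing yaw and roll.
; It applies rotations through a multicast event, with a DoOnce guarding against overlapping updates.
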(event Custom|TryRotate
  (params (NotifyData :type ST%20Notify%20Data%20Structure))
  ;[0 0.3517 1 0.82] Initializer
  (Networking|SwitchHasAuthority
    (:Authority
      (Utilities|FlowControl|DoOnce false :!label _label ; Don't overlap work if too fast.
        (:Completed
          (bind _keys (Utilities|Map|Keys (Variables|Default|GetstartingRotation)))
          (for _array_element _keys
            (Utilities|IsValid _array_element
              (:Is%20Valid
                (CallFunction|RotateDirectionalLight _array_element (Math|Rotator|MakeRotator 0.0 (+ (* (Utilities|Struct|BreakST_NotifyData_Day (Utilities|Struct|BreakST_NotifyData NotifyData)) 3.6e+02) (.pitch (.Value (Utilities|Map|Find (Variables|Default|GetstartingRotation) _array_element)))) 0.0)))))
          (goto _label Reset))))))

(event Custom|RotateDirectionalLight
  (params (DirectionalLight :type Directional%20Light%20Object%20Reference) (Rotation :type Rotator))
  ;[0 1 0.1542 0.82] RotateDirectionalLight (Multicast)
  (Transformation|SetActorRotation DirectionalLight Rotation))

(event EventBeginPlay
  ;[0 0.3517 1 0.82] Initializer
  (|CheckforTimeOfDayBP)
  (|CheckforPrimaryLight)
  (Utilities|FlowControl|Sequence
    (:then_0
      (if (Variables|TimeOfDay-SkyConfiguration|GetautoAlignSkyAtStart)
        (Utilities|FlowControl|Sequence
          (:then_0
            (Transformation|SetActorRotation (Variables|TimeOfDay-SkyConfiguration|GetLightSourceSun) "90.000000,180.000000,180.000000"))
          (:then_1
            (bind _lightsourcemoon (Variables|TimeOfDay-SkyConfiguration|GetLightSourceMoon)
              (:then
                (Transformation|SetActorRotation _lightsourcemoon "-90.000000, 0,0.000000"))
              (:else)))
          (:then_2
            (for _array_element (Utilities|Array|MakeArray (Variables|TimeOfDay-SkyConfiguration|GetLightSourceSun) (Variables|TimeOfDay-SkyConfiguration|GetLightSourceMoon)) :!label _label
              (Utilities|IsValid _array_element
                (:Is%20Valid
                  (Utilities|Map|Add (Variables|Default|GetstartingRotation) _array_element (Transformation|GetActorRotation _array_element)))))))
        (else
          (goto _label))))
    (:then_1
      (EventDispatchers|BindEventtoNotifyTime (Variables|TimeOfDay-SkyConfiguration|GetTimeOfDayBP) (delegate Custom|TryRotate)))))

(fn ConstructionScript)