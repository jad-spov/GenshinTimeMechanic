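; BP_TimeOfDay_Sounds swaps two sets of linked ambient sounds between day and night, following the world's BP_TimeOfDay clock.
; At BeginPlay it finds that clock, warns on screen if it or the sounds are missing, and binds to its time notifications.
; Each authority-side notification runs the daytime test, with paired DoOnce gates limiting switches to transitions.
; Multicast events then fade each set's audio components in or out.
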(event Custom|TrySounds
  (params (NotifyData :type ST%20Notify%20Data%20Structure))
  (bind _time (Utilities|Struct|BreakST_NotifyData NotifyData))
  (bind (_hour24 _minute _second) (Utilities|Struct|BreakST_NotifyData_Time _time))
  ;[0 0.3517 1 0.82] Initializer
  (Networking|SwitchHasAuthority
    (:Authority
      (if (.isDaytime (Default|IsTimeOfDay (Variables|TimeOfDay-AmbientSoundsConfiguration|GetTimeOfDayBP) _hour24 _minute _second (Variables|TimeOfDay-AmbientSoundsConfiguration|GetDaytimeStartAt) (Variables|TimeOfDay-AmbientSoundsConfiguration|GetNighttimeStartAt))) ; Is it daytime?
        (Utilities|FlowControl|DoOnce false :!label _label
          (:Completed
            (CallFunction|TurnonSounds (Variables|TimeOfDay-AmbientSoundsConfiguration|GetAmbientSoundsDay))
            (CallFunction|TurnOffSounds (Variables|TimeOfDay-AmbientSoundsConfiguration|GetAmbientSoundsNight))
            (goto _label_2 Reset)))
        (else
          (Utilities|FlowControl|DoOnce false :!label _label_2
            (:Completed
              (CallFunction|TurnonSounds (Variables|TimeOfDay-AmbientSoundsConfiguration|GetAmbientSoundsNight))
              (CallFunction|TurnOffSounds (Variables|TimeOfDay-AmbientSoundsConfiguration|GetAmbientSoundsDay))
              (goto _label Reset))))))))

(event Custom|TurnOffSounds
  (params (AmbientSounds :type Array%20of%20Ambient%20Sound%20Object%20References))
  ;[0 1 0.1542 0.82] Toggle Sounds (multicast)
  (for _array_element AmbientSounds
    (Utilities|IsValid _array_element
      (:Is%20Valid
        (Audio|Components|Audio|FadeOut (Variables|/Script/Engine.AmbientSound|GetAudioComponent _array_element) (Variables|TimeOfDay-AmbientSoundsConfiguration|GetFade%20out%20Duration) 0.0 "Linear" :!class /Script/Engine.AudioComponent)))))

(event Custom|TurnOnSounds
  (params (AmbientSounds :type Array%20of%20Ambient%20Sound%20Object%20References))
  ;[0 1 0.1542 0.82] Toggle Sounds (multicast)
  (for _array_element AmbientSounds
    (Utilities|IsValid _array_element
      (:Is%20Valid
        (Audio|Components|Audio|FadeIn (Variables|/Script/Engine.AmbientSound|GetAudioComponent _array_element) (Variables|TimeOfDay-AmbientSoundsConfiguration|GetFade%20in%20Duration) 1.0 0.0 "Linear" :!class /Script/Engine.AudioComponent)))))

(event EventBeginPlay
  (bind _timeofdaybp (Variables|TimeOfDay-AmbientSoundsConfiguration|GetTimeOfDayBP))
  ;[0 0.3517 1 0.82] Initializer
  (|CheckforTimeOfDayBP)
  (|CheckforAmbientSounds)
  (EventDispatchers|BindEventtoNotifyTime _timeofdaybp (delegate Custom|TrySounds))
  (if (.isDaytime (Default|IsTimeOfDay _timeofdaybp (.Hour24 (Utilities|Struct|BreakST_NotifyData_Time (Utilities|Struct|BreakST_NotifyData (stale Custom|TrySounds NotifyData)))) (.Minute (Utilities|Struct|BreakST_NotifyData_Time (Utilities|Struct|BreakST_NotifyData (stale Custom|TrySounds NotifyData)))) (.Second (Utilities|Struct|BreakST_NotifyData_Time (Utilities|Struct|BreakST_NotifyData (stale Custom|TrySounds NotifyData)))) (Variables|TimeOfDay-AmbientSoundsConfiguration|GetDaytimeStartAt) (Variables|TimeOfDay-AmbientSoundsConfiguration|GetNighttimeStartAt))) ; Is it daytime?
    (Utilities|FlowControl|DoOnce false :!label _label
      (:Completed
        (CallFunction|TurnonSounds (Variables|TimeOfDay-AmbientSoundsConfiguration|GetAmbientSoundsDay))
        (CallFunction|TurnOffSounds (Variables|TimeOfDay-AmbientSoundsConfiguration|GetAmbientSoundsNight))
        (goto _label_2 Reset)))
    (else
      (Utilities|FlowControl|DoOnce false :!label _label_2
        (:Completed
          (CallFunction|TurnonSounds (Variables|TimeOfDay-AmbientSoundsConfiguration|GetAmbientSoundsNight))
          (CallFunction|TurnOffSounds (Variables|TimeOfDay-AmbientSoundsConfiguration|GetAmbientSoundsDay))
          (goto _label Reset))))))

(fn ConstructionScript)