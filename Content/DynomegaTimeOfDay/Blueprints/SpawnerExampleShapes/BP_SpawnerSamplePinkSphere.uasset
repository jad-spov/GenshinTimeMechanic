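; BP_SpawnerSamplePinkSphere is a sample shape, presumably for spawner demonstrations, that pops upward and animates its scale when it appears.
; On BeginPlay, the authority calls the Spawner event, commented as multicast, which launches the static mesh with a velocity-change impulse and plays a quiet, randomly pitched sound.
; The authority also runs a timeline that drives the mesh's uniform world scale.
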(event Custom|Spawner
  ;[0 1 0.1542 0.82] Spawner Effects (multicast)
  (Physics|AddImpulse (Variables|Default|GetStaticMesh) "0, 0,1000.000000" "None" true)
  (Audio|PlaySoundatLocation "/Engine/VREditor/Sounds/UI/Dockable_Window_Pick_Up.Dockable_Window_Pick_Up" (Transformation|GetWorldLocation (Variables|Default|GetStaticMesh)) "0, 0, 0" 0.1 (Math|Random|RandomFloatinRange 0.5 1.0) 0.0 0 0 0 0))

(event EventBeginPlay
  ;[0 0.3517 1 0.82] Initializer
  (Networking|SwitchHasAuthority
    (:Authority
      (CallFunction|Spawner)
      (bind _newtrack_0 (Timeline|Timeline_0 PlayFromStart)
        (:Update
          (Transformation|SetWorldScale3D (Variables|Default|GetStaticMesh) (Math|Vector|MakeVector _newtrack_0 _newtrack_0 _newtrack_0)))))))

(fn ConstructionScript)