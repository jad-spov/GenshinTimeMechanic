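; BP_SpawnerSampleSilverSphere is an example spawnable physics sphere that turns into a magic cone once enough copies accumulate.
; On BeginPlay the authority runs the Spawner effect, commented as multicast, which launches the sphere upward with a sound.
; It then counts all silver spheres; at ten or more it spawns a scaled-up BP_SpawnerSampleMagicCone and gives spheres without a lifespan a short one plus a stronger upward impulse.
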(event Custom|Spawner
  ;[0 1 0.1542 0.82] Spawner Effects (multicast)
  (Physics|AddImpulse (Variables|Default|GetStaticMesh) "0,0.000000,600.000000" "None" true)
  (Audio|SpawnSoundatLocation "/Engine/VREditor/Sounds/UI/Enter_Play.Enter_Play" (Transformation|GetActorLocation) "0, 0, 0" 1.0 1.0 0.0 0 0))

(event Custom|FinalImpulseEffect
  (params (Actor :type BP%20Spawner%20Sample%20Silver%20Sphere%20Object%20Reference))
  ;[0 1 0.1542 0.82] Despawn Effect
  (Physics|AddImpulse (Variables|BP_SpawnerSampleSilverSphere_C|GetStaticMesh Actor) "0,0.000000,3600.000000" "None" true))

(event EventBeginPlay
  ;[0 0.3517 1 0.82] Initializer
  (Networking|SwitchHasAuthority
    (:Authority
      (CallFunction|Spawner)
      (bind _outactors (Actor|GetAllActorsOfClass "BP_SpawnerSampleSilverSphere_C"))
      (if (> (Utilities|Array|Length _outactors) 9)
        (Game|SpawnActorfromClass "/Game/DynomegaTimeOfDay/Blueprints/SpawnerExampleShapes/BP_SpawnerSampleMagicCone.BP_SpawnerSampleMagicCone_C" (Math|Transform|MakeTransform (Transformation|GetActorLocation) (Transformation|GetActorRotation) "3.000000,3.000000,3.000000") "Undefined" 0 0)
        (for _array_element _outactors
          (if (== (Actor|GetLifeSpan _array_element) 0.0)
            (Actor|SetLifeSpan _array_element 1.0)
            (CallFunction|FinalImpulseEffect _array_element)))))))

(fn ConstructionScript)